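; BP_LevelMG is a level manager that handles level transition requests and holds shared status data for the player, enemy and results.
; Level_Trans passes an index to LevelChange, which range-checks it against LevelName and only prints that name, as the Open Level node is unconnected.
; Getters expose default player and enemy status with flip distance and low/high flip power.
; Result statuses live in an auto-sizing indexed array, readable singly or whole.
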(event Custom|Level_Trans
  (params (inLevelNum :type SceneName%20Enum :default "NewEnumerator0"))
  (CallFunction|LevelChange inLevelNum))

(fn LevelChange
  (params (SceneName :type SceneName%20Enum :default "NewEnumerator0"))
  (bind _returnvalue (Math|Conversions|ToInteger(Byte) SceneName))
  (bind _levelname (Variables|Default|GetLevelName))
  (if (Math|Integer|InRange(Integer) _returnvalue 0 (Utilities|Array|Length _levelname))
    (Development|PrintString (Utilities|Array|Get(acopy) _levelname _returnvalue))))

(fn GetDefaultEnemyStatus
  (bind _defaultenemystatus (Variables|Default|GetDefaultEnemyStatus))
  (return (.flipdisstatus _defaultenemystatus) (.lowflippow _defaultenemystatus) (.highflippow _defaultenemystatus) (Variables|Default|GetDefaultEnemyStatus)))

(fn GetDefaultPlayerStatus
  (bind _defaultplayerstatus (Variables|Default|GetDefaultPlayerStatus))
  (return (.flipdisstatus _defaultplayerstatus) (.lowflippow _defaultplayerstatus) (.highflippow _defaultplayerstatus) (Variables|Default|GetDefaultPlayerStatus)))

(fn SetResultStatus
  (params (inValue :type Integer) (inStatus :type Game%20Result%20Status%20Structure))
  (Utilities|Array|SetArrayElem (Variables|Default|GetResultStatus) inValue inStatus true))

(fn GetArrayResultStatus
  (return (Variables|Default|GetResultStatus)))

(fn GetResultStatus
  (params (inValue :type Integer))
  (return (Utilities|Array|Get(acopy) (Variables|Default|GetResultStatus) inValue)))