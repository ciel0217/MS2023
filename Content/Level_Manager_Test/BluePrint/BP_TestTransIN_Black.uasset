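; BP_TestTransIN_Black is a screen transition that plays on spawn and then changes level.
; On BeginPlay it adds a WBP_TransTest widget to the viewport and resets its own CustomTimeDilation.
; A timeline drives the "Offset" scalar of the widget's RetainerBox effect material to animate the transition.
; When finished, if that material is valid, it removes the widget and passes SceneName to LevelChange on the BP_LevelMG GameInstance.
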(event EventBeginPlay
  (Variables|Default|SetGameInstance (Game|GetGameInstance))
  (Utilities|FlowControl|Sequence
    (:then_0
      (bind _returnvalue (UserInterface|CreateWidget "/Game/kawada/WIdget/WBP_TransTest.WBP_TransTest_C"))
      (bind _output_get (Variables|Default|SetWigetTrans _returnvalue))
      (UserInterface|Viewport|AddtoViewport _output_get 0)
      (Variables|Default|SetCustomTimeDilation 1.0))
    (:then_1
      (bind _新規track_0 (Timeline|TimeLine Play)
        (:Update
          (Utilities|IsValid (Class|RetainerBox|GetEffectMaterial (Variables|/Game/kawada/WIdget/WBP_TransTest.WBP_TransTest_C|GetRetainerBox_51 (Variables|Default|GetWigetTrans)))
            (:Is%20Valid
              (Rendering|Material|SetScalarParameterValue (Class|RetainerBox|GetEffectMaterial (Variables|/Game/kawada/WIdget/WBP_TransTest.WBP_TransTest_C|GetRetainerBox_51 (Variables|Default|GetWigetTrans))) "Offset" _新規track_0 :!class /Script/Engine.MaterialInstanceDynamic))))
        (:Finished
          (Utilities|IsValid (Class|RetainerBox|GetEffectMaterial (Variables|/Game/kawada/WIdget/WBP_TransTest.WBP_TransTest_C|GetRetainerBox_51 (Variables|Default|GetWigetTrans)))
            (:Is%20Valid
              (Widget|RemovefromParent _output_get)
              (Utilities|IsValid (Variables|Default|GetGameInstance)
                (:Is%20Valid
                  (bind _asbp_level_mg (Utilities|Casting|CastToBP_LevelMG (Variables|Default|GetGameInstance)))
                  (Default|LevelChange _asbp_level_mg (Variables|Default|GetSceneName)))))))))))

(fn ConstructionScript)