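; BP_StAIEnemy is an AI enemy pawn that reports its hit state to its Blackboard on overlap.
; Begin overlap runs the parent logic, halts FloatingPawnMovement immediately, then copies IsHit into the Hit key.
; End overlap runs the parent logic and refreshes the same key without stopping movement.
; BeginPlay, Tick and construction only call the parent implementations.
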(event EventBeginPlay
  (|CallParentFunction))

(event Collision|EventActorBeginOverlap
  (params (OtherActor :type Actor%20Object%20Reference))
  (|CallParentFunction OtherActor)
  (Components|Movement|StopMovementImmediately (Variables|Default|GetFloatingPawnMovement))
  (AI|Components|Blackboard|SetValueasBool (AI|GetBlackboard 0) (Variables|Default|GetHit) (Variables|Default|GetisHit)))

(event EventTick
  (params (DeltaSeconds :type Float%20%28single-precision%29))
  (|CallParentFunction DeltaSeconds))

(event Collision|EventActorEndOverlap
  (params (OtherActor :type Actor%20Object%20Reference))
  (|CallParentFunction OtherActor)
  (AI|Components|Blackboard|SetValueasBool (AI|GetBlackboard 0) (Variables|Default|GetHit) (Variables|Default|GetisHit)))

(fn ConstructionScript
  (|CallParentFunction))