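; BP_RotUpItem+1 is an item Blueprint that, going by its name, is a +1 rotation upgrade, raising a status on the actor that hits it.
; Its Hit override runs the parent logic, then calls AddStatus on that actor with the StatusName and StatusValue variables.
; The event graph holds only disabled placeholder events, and the construction script just calls its parent.
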(event EventBeginPlay
  (|CallParentFunction) ; このノードは無効になっているため呼び出せません。\n機能をビルドするにはピンをドラッグしてください。
)

(event Collision|EventActorBeginOverlap
  (params (OtherActor :type Actor%20Object%20Reference))
  (|CallParentFunction OtherActor) ; このノードは無効になっているため呼び出せません。\n機能をビルドするにはピンをドラッグしてください。
)

(event EventTick
  (params (DeltaSeconds :type Float%20%28single-precision%29))
  (|CallParentFunction DeltaSeconds) ; このノードは無効になっているため呼び出せません。\n機能をビルドするにはピンをドラッグしてください。
)

(fn ConstructionScript
  (|CallParentFunction))

(fn Hit
  (params (inActor :type BP%20Object%20Actor%20Object%20Reference))
  (|CallParentFunction inActor)
  (Default|AddStatus inActor (Variables|Default|GetStatusName) (Variables|Default|GetStatusValue)))