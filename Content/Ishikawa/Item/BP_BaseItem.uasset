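; BP_BaseItem is a base item actor that destroys itself when its Sphere overlaps a BP_ObjectActor; Hit's add-item calls are disconnected.
; When a BP_ObjectActor enters AcquisitionRange, a looping timer line-traces toward it and, once unobstructed, starts timed interpolated movement toward it.
; After a short delay, its Box picks up AreaNum from overlapping BP_AreaStatickMesh, used in handling BP_GameMode's area-delete event to destroy the item.
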(event OnComponentBeginOverlap(Sphere)
  (params (OverlappedComponent :type Primitive%20Component%20Object%20Reference) (OtherActor :type Actor%20Object%20Reference) (OtherComp :type Primitive%20Component%20Object%20Reference) (OtherBodyIndex :type Integer) (bFromSweep :type Boolean) (SweepResult :type Hit%20Result%20Structure%20%28by%20ref%29))
  ;[1 1 1] 取得処理
  (bind _asbp_object_actor (Utilities|Casting|CastToBP_ObjectActor OtherActor))
  (CallFunction|Hit _asbp_object_actor))

(event OnComponentBeginOverlap(AcquisitionRange)
  (params (OverlappedComponent :type Primitive%20Component%20Object%20Reference) (OtherActor :type Actor%20Object%20Reference) (OtherComp :type Primitive%20Component%20Object%20Reference) (OtherBodyIndex :type Integer) (bFromSweep :type Boolean) (SweepResult :type Hit%20Result%20Structure%20%28by%20ref%29))
  ;[1 1 1] 吸着範囲に入ったか？
  (Utilities|IsValid OtherActor
    (:Is%20Valid
      (Utilities|Casting|CastToBP_ObjectActor OtherActor)
      (Variables|Default|SetHit%20Other%20Actor OtherActor)
      (bind _returnvalue (Utilities|Time|SetTimerbyFunctionName 0 "ObstacleTraceCheck" 0.1 true))
      (Variables|Default|SetObstacleTraceCheck_Handle _returnvalue))))

(event OnComponentEndOverlap(AcquisitionRange)
  (params (OverlappedComponent :type Primitive%20Component%20Object%20Reference) (OtherActor :type Actor%20Object%20Reference) (OtherComp :type Primitive%20Component%20Object%20Reference) (OtherBodyIndex :type Integer))
  ;[1 1 1] 範囲外に出た場合トレースの終了
  (Utilities|IsValid OtherActor
    (:Is%20Valid
      (if (== OtherActor (Variables|Default|GetHit%20Other%20Actor))
        (Utilities|Time|ClearandInvalidateTimerbyHandle (Variables|Default|GetObstacleTraceCheck_Handle))))))

(event OnComponentBeginOverlap(Box)
  (params (OverlappedComponent :type Primitive%20Component%20Object%20Reference) (OtherActor :type Actor%20Object%20Reference) (OtherComp :type Primitive%20Component%20Object%20Reference) (OtherBodyIndex :type Integer) (bFromSweep :type Boolean) (SweepResult :type Hit%20Result%20Structure%20%28by%20ref%29))
  (bind _asbp_area_statick_mesh (Utilities|Casting|CastToBP_AreaStatickMesh OtherActor))
  (CallFunction|SetAreaNum (Variables|/Game/Ishikawa/BP_AreaStatickMesh.BP_AreaStatickMesh_C|GetAreaNum _asbp_area_statick_mesh)))

(event Custom|Adsorb
  ;[1 1 1] 吸着
  (Transformation|SetActorLocation (Math|Interpolation|VInterpTo (Transformation|GetActorLocation) (Transformation|GetActorLocation (Variables|Default|GetHit%20Other%20Actor)) (Utilities|Time|GetWorldDeltaSeconds) (Variables|Default|GetAbsord%20Interp%20Speed)) false false))

(event Custom|ObstacleTraceCheck
  ;[1 1 1] 他のオブジェクトに遮られてないか
  (bind _returnvalue (Class|KismetSystemLibrary|LineTraceMultiforObjects (+ (Transformation|GetActorLocation) "0.000000,0.000000,50.000000") (Transformation|GetActorLocation (Variables|Default|GetHit%20Other%20Actor)) (Variables|Default|GetObject%20Types) false 0 "None" true))
  (if (not _returnvalue)
    (bind _returnvalue_2 (Utilities|Time|SetTimerbyFunctionName 0 "Adsorb" 0.01 true))
    (Variables|Default|SetAdsorb%20to%20Actor_Handle _returnvalue_2)))

(event Custom|AreaDelete
  (params (AreaNum :type Integer))
  (if (== AreaNum (Variables|Default|GetAreaNum))
    (Actor|DestroyActor)))

(event EventBeginPlay
  (bind _box (Variables|Default|GetBox))
  (Collision|SetCollisionEnabled _box "NoCollision")
  (Utilities|FlowControl|Delay 0.2)
  (Collision|SetCollisionEnabled _box "QueryOnly")
  (bind _asbp_game_mode (Utilities|Casting|CastToBP_GameMode (Game|GetGameMode)))
  (EventDispatchers|BindEventtoAreaDelete _asbp_game_mode (delegate Custom|AreaDelete)))

(event Collision|EventActorBeginOverlap
  (params (OtherActor :type Actor%20Object%20Reference)))

(event EventTick
  (params (DeltaSeconds :type Float%20%28single-precision%29))
  ;[1 1 1] 回転
)

(fn ConstructionScript)

(fn GetMesh
  (return 0))

(fn SetAreaNum
  (params (AreaNum :type Integer))
  (Variables|Default|SetAreaNum AreaNum))

(fn Hit
  (params (inActor :type BP%20Object%20Actor%20Object%20Reference))
  (Actor|DestroyActor))