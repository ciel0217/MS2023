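; Item spawner that scatters random pickups from ItemClasses across the level when play begins.
; BeginPlay grabs the first BlockingVolume found as the spawn area, then SpawnItem loops based on ItemSum.
; Each item spawns at a random reachable navmesh point within a radius equal to the volume's larger horizontal extent, so placement can fall outside the box.
; Spawn height is fixed, and collisions never block spawning.
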(event EventBeginPlay
  (bind _returnvalue (Actor|GetActorOfClass "/Script/Engine.BlockingVolume"))
  (Variables|Default|SetBoxVolume _returnvalue)
  (CallFunction|SpawnItem))

(event Collision|EventActorBeginOverlap
  (params (OtherActor :type Actor%20Object%20Reference)))

(event EventTick
  (params (DeltaSeconds :type Float%20%28single-precision%29)))

(fn ConstructionScript)

(fn SpawnItem
  (bind _boxvolume (Variables|Default|GetBoxVolume))
  (bind (_origin _boxextent) (Collision|GetActorBounds _boxvolume false false))
  (bind _returnvalue (Math|Float|Max(Float) (.x _boxextent) (.y _boxextent)))
  (bind _randomlocation (AI|Navigation|GetRandomReachablePointinRadius _origin _returnvalue 0 0))
  (bind _returnvalue_2 (Math|Conversions|ToTransform(Vector) _randomlocation))
  (for _index (range 0 (Variables|Default|GetItemSum))
    (Game|SpawnActorfromClass (.OutItem (Utilities|Array|Random (Variables|Default|GetItemClasses))) (Math|Transform|MakeTransform (Math|Vector|MakeVector (.x (.location _returnvalue_2)) (.y (.location _returnvalue_2)) 1e+02) (.rotation _returnvalue_2) (.scale _returnvalue_2)) "AlwaysSpawn" "MultiplyWithRoot" 0 0)))