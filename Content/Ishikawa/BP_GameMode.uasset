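; Game mode for a timed, round-based survival match in which areas are deleted as rounds end.
; BeginPlay plays an intro level sequence, then blends the camera to the player and signals game start.
; Tick drives the round clock, using resettable DoOnce gates to announce each area's pending deletion, delete it and advance, ending the game in the last round.
; An actor counter triggers a level transition through BP_LevelMG when one or fewer remain.
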(event EventBeginPlay
  (Variables|Default|SetGameInstance_Handle (Game|GetGameInstance))
  (CallFunction|InitParRound)
  (bind _returnvalue (Game|SpawnActorfromClass :Class "/Script/LevelSequence.LevelSequenceActor" :CollisionHandlingOverride "AlwaysSpawn" :TransformScaleMethod "MultiplyWithRoot" :LevelSequenceAsset "/Game/okada/GameStartS.GameStartS" :Instigator 0))
  (Utilities|IsValid _returnvalue
    (:Is%20Valid
      (Variables|Default|SetLevelSequence _returnvalue)
      (Game|Player|SetViewTargetwithBlend (Game|GetPlayerController 0) 0 0.0 "VTBlend_Linear" 0.0 false))
    (:Is%20Not%20Valid
      _))
  (Utilities|FlowControl|Delay 0.01)
  (Default|CallStart)
  (Utilities|IsValid (Variables|Default|GetLevelSequence)
    (:Is%20Valid
      (Sequencer|Player|Play (Variables|/Script/LevelSequence.LevelSequenceActor|GetSequencePlayer (Variables|Default|GetLevelSequence)) :!class /Script/MovieScene.MovieSceneSequencePlayer)
      (Utilities|FlowControl|Delay 5.5)
      (bind _returnvalue_2 (Actor|GetActorOfClass "/Game/kawada/testBP/TestMoveObject/BP_ObjectActor_Player.BP_ObjectActor_Player_C"))
      (Utilities|IsValid _returnvalue_2
        (:Is%20Valid
          (Game|Player|SetViewTargetwithBlend (Game|GetPlayerController 0) _returnvalue_2 0.2 "VTBlend_Linear" 0.0 false)
          (Default|CallGameStart))))))

(event EventTick
  (params (DeltaSeconds :type Float%20%28single-precision%29))
  (bind _currentroundnum (Variables|Default|GetCurrentRoundNum))
  (bind _roundtoroundtimesecnods (Variables|Default|GetRoundToRoundTimeSecnods))
  (bind _currentroundnum_2 (Variables|Default|GetCurrentRoundNum))
  (bind _currentroundnum_3 (Variables|Default|GetCurrentRoundNum))
  (bind _returnvalue (* _currentroundnum _roundtoroundtimesecnods))
  (if (not (Variables|Default|GetIsGameSet))
    (bind _output_get (Variables|Default|SetCurrentTimeSeconds (+ DeltaSeconds (Variables|Default|GetCurrentTimeSeconds))))
    (if (> _output_get (- _returnvalue (Variables|Default|GetDeleteAreaTimeSeconds)))
      (if (== (Variables|Default|GetCurrentRoundNum) (Variables|Default|GetRoundSum))
        (Development|PrintString "GameSet")
        (Default|CallGameSet)
        (Variables|Default|SetIsGameSet true)
        (else
          (Utilities|FlowControl|Sequence
            (:then_0
              (Utilities|FlowControl|DoOnce false :!label _label
                (:Completed
                  (Default|CallAreaDeleteStart _currentroundnum_2 (Variables|Default|GetDeleteAreaTimeSeconds))
                  (Development|PrintString "DeleteStart"))))
            (:then_1
              (if (> _output_get _returnvalue)
                (Utilities|FlowControl|DoOnce false :!label _label_2
                  (:Completed
                    (Default|CallAreaDelete _currentroundnum_2)
                    (Math|Integer|IncrementInt _currentroundnum_3
                      (:%20%20
                        (if (not (> (Variables|Default|GetCurrentRoundNum) (Variables|Default|GetRoundSum)))
                          (Utilities|FlowControl|Sequence
                            (:then_0
                              (goto _label Reset))
                            (:then_1
                              (goto _label_2 Reset))
                            (:then_2
                              (Default|CallStartPerRound _currentroundnum_3))))))))))))))))

(fn ConstructionScript)

(fn InitParRound
  (Variables|Default|SetCurrentTimeSeconds 0.0)
  (bind _output_get (Variables|Default|SetCurrentRoundNum 1))
  (Default|CallStartPerRound _output_get))

(fn ActorDead
  (bind _result (Math|Integer|DecrementInt (Variables|Default|GetActorNum))
    (:%20%20
      (if (<= _result 1)
        (bind _asbp_level_mg (Utilities|Casting|CastToBP_LevelMG (Variables|Default|GetGameInstance_Handle)))
        (Default|LevelTrans _asbp_level_mg "NewEnumerator1")))))

(fn AwakeActor
  (Math|Integer|IncrementInt (Variables|Default|GetActorNum)))