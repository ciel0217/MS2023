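; BP_AreaManager is a manager actor that deletes numbered areas when the game mode signals it.
; On BeginPlay it casts the game mode to BP_GameMode and binds its AreaDelete and AreaDeleteStart events.
; AreaDelete converts the one-based area number to a clamped index into its Areas array and calls DeleteArea on that entry.
; The AreaDeleteStart handler is bound but empty.
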(event Custom|AreaDelete
  (params (AreaNum :type Integer))
  (bind _areas (Variables|Default|GetAreas))
  (Default|DeleteArea (Utilities|Array|Get(acopy) _areas (Math|Integer|Clamp(Integer) (- AreaNum 1) 0 (- (Utilities|Array|Length _areas) 1)))))

(event Custom|AreaDeleteStart
  (params (AreaNum :type Integer) (AreaToDeleteSecond :type Float%20%28double-precision%29)))

(event EventBeginPlay
  (bind _asbp_game_mode (Utilities|Casting|CastToBP_GameMode (Game|GetGameMode)))
  (EventDispatchers|BindEventtoAreaDelete _asbp_game_mode (delegate Custom|AreaDelete))
  (EventDispatchers|BindEventtoAreaDeleteStart _asbp_game_mode (delegate Custom|AreaDeleteStart)))

(event EventTick
  (params (DeltaSeconds :type Float%20%28single-precision%29)))

(fn ConstructionScript)