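; Test actor that spins around world Z while rocking up and down in a sine-driven pitch swing.
; Each Tick turns the right vector by a fixed step, rebuilds a level forward vector from it, and tilts that around the right axis by the sine of accumulated time.
; MakeRotFromXY rebuilds the rotation from both axes.
; The yaw step is per frame, so spin speed depends on frame rate.
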(event EventBeginPlay
  (Variables|Default|SetTIme 0.0))

(event Collision|EventActorBeginOverlap
  (params (OtherActor :type Actor%20Object%20Reference)))

(event EventTick
  (params (DeltaSeconds :type Float%20%28single-precision%29))
  (bind _returnvalue (Transformation|GetActorRightVector))
  (bind _returnvalue_2 (Math|Vector|RotateVectorAroundAxis _returnvalue 1.0 "0.000000,0.000000,1.000000"))
  (bind _output_get (Variables|Default|SetTIme (+ DeltaSeconds (Variables|Default|GetTIme))))
  (Transformation|SetActorRotation (Math|Rotator|MakeRotfromXY (Math|Vector|RotateVectorAroundAxis (Math|Rotator|GetRotationXVector (Class|KismetMathLibrary|MakeRotfromYZ _returnvalue_2 (Math|Vector|MakeVector 0.0 0.0 1.0))) (* (Math|Trig|Sin(Radians) _output_get) 6e+01) _returnvalue_2) _returnvalue_2)))

(fn ConstructionScript)