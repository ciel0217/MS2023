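; Minimap helper Blueprint that fits the level's BlockingVolume to the horizontal extent of static mesh geometry.
; CalcBlockingVolume scans all actors except BP_CreateMapTexture, using root-child static mesh bounds to grow Min and Max only when both X and Y exceed the current corner.
; It moves the found volume to the XY midpoint at a fixed height and sets its brush's bounds scale from the X span alone.
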(event Custom|CalcBlockingVolume
  (bind _returnvalue (Actor|GetActorOfClass "/Script/Engine.BlockingVolume"))
  (Variables|Default|SetBlockingVolume _returnvalue)
  (bind _outactors (Actor|GetAllActorsOfClass "/Script/Engine.Actor"))
  (for _array_element _outactors
    (Utilities|Casting|CastToBP_CreateMapTexture _array_element
      (:CastFailed
        (for _array_element_2 (Components|GetChildrenComponents (Variables|/Script/Engine.Actor|GetRootComponent _array_element) true)
          (bind _asstatic_mesh_component (Utilities|Casting|CastToStaticMeshComponent _array_element_2))
          (if (and (< (.x (- (.Origin (Collision|GetComponentBounds _asstatic_mesh_component)) (.BoxExtent (Collision|GetComponentBounds _asstatic_mesh_component)))) (.x (Variables|Default|GetMin))) (< (.y (- (.Origin (Collision|GetComponentBounds _asstatic_mesh_component)) (.BoxExtent (Collision|GetComponentBounds _asstatic_mesh_component)))) (.y (Variables|Default|GetMin))))
            (Variables|Default|SetMin (Math|Vector|MakeVector (.x (- (.Origin (Collision|GetComponentBounds _asstatic_mesh_component)) (.BoxExtent (Collision|GetComponentBounds _asstatic_mesh_component)))) (.y (- (.Origin (Collision|GetComponentBounds _asstatic_mesh_component)) (.BoxExtent (Collision|GetComponentBounds _asstatic_mesh_component)))) 0.0)))
          (if (and (> (.x (+ (.Origin (Collision|GetComponentBounds _asstatic_mesh_component)) (.BoxExtent (Collision|GetComponentBounds _asstatic_mesh_component)))) (.x (Variables|Default|GetMax))) (> (.y (+ (.Origin (Collision|GetComponentBounds _asstatic_mesh_component)) (.BoxExtent (Collision|GetComponentBounds _asstatic_mesh_component)))) (.y (Variables|Default|GetMax))))
            (Variables|Default|SetMax (Math|Vector|MakeVector (.x (+ (.Origin (Collision|GetComponentBounds _asstatic_mesh_component)) (.BoxExtent (Collision|GetComponentBounds _asstatic_mesh_component)))) (.y (+ (.Origin (Collision|GetComponentBounds _asstatic_mesh_component)) (.BoxExtent (Collision|GetComponentBounds _asstatic_mesh_component)))) 0.0)))))))
  (Transformation|SetActorLocation (Variables|Default|GetBlockingVolume) (Math|Vector|MakeVector (.x (+ (/ (- (Variables|Default|GetMax) (Variables|Default|GetMin)) 2.0) (Variables|Default|GetMin))) (.y (+ (/ (- (Variables|Default|GetMax) (Variables|Default|GetMin)) 2.0) (Variables|Default|GetMin))) 2e+02) false false)
  (Rendering|SetBoundsScale (Variables|/Script/Engine.Brush|GetBrushComponent (Variables|Default|GetBlockingVolume)) (- (.x (Variables|Default|GetMax)) (.x (Variables|Default|GetMin)))))

(event Collision|EventActorBeginOverlap
  (params (OtherActor :type Actor%20Object%20Reference)))

(fn ConstructionScript)