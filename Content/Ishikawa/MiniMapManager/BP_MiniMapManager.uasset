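; BP_MiniMapManager creates the minimap widget and keeps its map imagery in step with area deletion events from BP_GameMode.
; On BeginPlay it has CreateMap capture the map, then feeds the render results into numbered texture parameters on the widget's dynamic material.
; While an area is being deleted, Tick pulses that area's channel of the AreaCheck vector parameter with an absolute sine.
; Completed deletion triggers a recapture and texture refresh.
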(event Custom|AreaDelete
  (params (AreaNum :type Integer))
  (Variables|Default|SetIsDeleteArea false)
  (Variables|Default|SetDeleteTime 0.0)
  (Variables|Default|SetDeleteAreaNum 0)
  (Default|TakeCapture (Variables|Default|GetCreateMap))
  (CallFunction|SetMiniMapTexture))

(event Custom|AreaDeleteStart
  (params (AreaNum :type Integer) (AreaToDeleteCompleteSecond :type Float%20%28double-precision%29))
  (Variables|Default|SetIsDeleteArea true)
  (Variables|Default|SetDeleteAreaNum AreaNum))

(event EventBeginPlay
  (bind _asbp_game_mode (Utilities|Casting|CastToBP_GameMode (Game|GetGameMode)))
  (EventDispatchers|BindEventtoAreaDeleteStart _asbp_game_mode (delegate Custom|AreaDeleteStart))
  (EventDispatchers|BindEventtoAreaDelete _asbp_game_mode (delegate Custom|AreaDelete))
  (bind _returnvalue (UserInterface|CreateWidget "/Game/Ishikawa/Widget/BPW_MiniMap.BPW_MiniMap_C"))
  (bind _output_get (Variables|Default|SetMiniMapWidget _returnvalue))
  (UserInterface|Viewport|AddtoViewport _output_get 0)
  (CallFunction|CreateandSetMiniMapTexture))

(event Collision|EventActorBeginOverlap
  (params (OtherActor :type Actor%20Object%20Reference)))

(event EventTick
  (params (DeltaSeconds :type Float%20%28single-precision%29))
  (if (Variables|Default|GetIsDeleteArea)
    (Variables|Default|SetDeleteTime (+ DeltaSeconds (Variables|Default|GetDeleteTime)))
    (CallFunction|CalcDeleteArea)))

(fn ConstructionScript)

(fn CreateandSetMiniMapTexture
  (Default|StartTakeCaptureandExport (Variables|Default|GetCreateMap))
  (CallFunction|SetMiniMapTexture))

(fn CalcDeleteArea
  (bind _deletetime (Variables|Default|GetDeleteTime))
  (bind _deleteareanum (Variables|Default|GetDeleteAreaNum))
  (bind _returnvalue (Math|Trig|Sin(Radians) _deletetime))
  (bind _returnvalue_2 (Math|Float|Absolute(Float) _returnvalue))
  (if (== _deleteareanum 1)
    (LocalVariables|SetParameter (Utilities|Struct|MakeLinearColor _returnvalue_2 0.0 0.0 0.0))
    (bind _returnvalue_3 (Appearance|GetDynamicMaterial (Variables|/Game/Ishikawa/Widget/BPW_MiniMap.BPW_MiniMap_C|GetBack (Variables|Default|GetMiniMapWidget)) :!class /Script/UMG.Image :!label _label))
    (Rendering|Material|SetVectorParameterValue _returnvalue_3 "AreaCheck" (LocalVariables|GetParameter) :!class /Script/Engine.MaterialInstanceDynamic)
    (elif (== _deleteareanum 2)
      (LocalVariables|SetParameter (Utilities|Struct|MakeLinearColor 0.0 _returnvalue_2 0.0 0.0))
      (goto _label)
      (elif (== _deleteareanum 3)
        (LocalVariables|SetParameter (Utilities|Struct|MakeLinearColor 0.0 0.0 _returnvalue_2 0.0))
        (goto _label)
        (elif (== _deleteareanum 4)
          (LocalVariables|SetParameter (Utilities|Struct|MakeLinearColor 0.0 0.0 0.0 _returnvalue_2))
          (goto _label))))))

(fn SetMiniMapTexture
  (for (_array_element _array_index) (Variables|/Game/Ishikawa/MiniMapManager/CreateMapTexture/BP_CreateMapTexture.BP_CreateMapTexture_C|GetRenderMaterials (Variables|Default|GetCreateMap))
    (bind _returnvalue (Appearance|GetDynamicMaterial (Variables|/Game/Ishikawa/Widget/BPW_MiniMap.BPW_MiniMap_C|GetBack (Variables|Default|GetMiniMapWidget)) :!class /Script/UMG.Image))
    (Rendering|Material|SetTextureParameterValue _returnvalue (Utilities|String|StringToName (Utilities|String|Append (LocalVariables|GetParameterName) (Utilities|String|ToString(Integer) (+ _array_index 1)))) _array_element)))