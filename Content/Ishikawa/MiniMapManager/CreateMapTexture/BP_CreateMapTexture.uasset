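; BP_CreateMapTexture is an editor-placed capture actor that renders map area textures for the minimap.
; On construction it centers itself above the first BlockingVolume and sizes its orthographic camera and scene capture from the volume's bounds.
; StartTakeCaptureAndExport creates one render target per GameMode RoundSum, then captures each Areas actor in isolation via ShowOnlyActors.
; Only the capture component's current target, the last one captured, is exported to disk.
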(event Custom|StartTakeCaptureAndExport
  (CallFunction|CreateRenderMaterial)
  (CallFunction|TakeCapture)
  (CallFunction|ExportSceneTexture (Variables|Default|GetFile%20Path) (Variables|Default|GetFile%20Name)))

(event EventBeginPlay)

(event Collision|EventActorBeginOverlap
  (params (OtherActor :type Actor%20Object%20Reference)))

(event EventTick
  (params (DeltaSeconds :type Float%20%28single-precision%29)))

(fn ConstructionScript
  (CallFunction|UpdateSceneCaptureSetting))

(fn UpdateSceneCaptureSetting
  (bind _returnvalue (Actor|GetActorOfClass "/Script/Engine.BlockingVolume"))
  (Transformation|SetActorLocation (Math|Vector|MakeVector (.x (.Origin (Collision|GetActorBounds _returnvalue false false))) (.y (.Origin (Collision|GetActorBounds _returnvalue false false))) (* (Math|Float|Max(Float) (.x (.BoxExtent (Collision|GetActorBounds _returnvalue false false))) (.y (.BoxExtent (Collision|GetActorBounds _returnvalue false false)))) 2.0)) false false)
  (Class|CameraComponent|SetOrthoWidth (Variables|Default|GetCamera) (* (Math|Float|Max(Float) (.x (.BoxExtent (Collision|GetActorBounds _returnvalue false false))) (.y (.BoxExtent (Collision|GetActorBounds _returnvalue false false)))) 2.0))
  (Variables|/Script/Engine.SceneCaptureComponent2D|SetOrthoWidth (Variables|Default|GetSceneCaptureComponent2D) (* (Math|Float|Max(Float) (.x (.BoxExtent (Collision|GetActorBounds _returnvalue false false))) (.y (.BoxExtent (Collision|GetActorBounds _returnvalue false false)))) 2.0)))

(fn TakeCapture
  (bind _scenecapturecomponent2d (Variables|Default|GetSceneCaptureComponent2D))
  (for (_array_element _array_index) (Variables|Default|GetAreas)
    (Variables|/Script/Engine.SceneCaptureComponent|SetShowOnlyActors _scenecapturecomponent2d (Utilities|Array|MakeArray _array_element))
    (Variables|/Script/Engine.SceneCaptureComponent2D|SetTextureTarget _scenecapturecomponent2d (Utilities|Array|Get(acopy) (Variables|Default|GetRenderMaterials) _array_index))
    (Rendering|SceneCapture|CaptureScene _scenecapturecomponent2d :!class /Script/Engine.SceneCaptureComponent2D)))

(fn ExportSceneTexture
  (params (FilePath :type String) (FileName :type String))
  (Rendering|ExportRenderTarget (Variables|/Script/Engine.SceneCaptureComponent2D|GetTextureTarget (Variables|Default|GetSceneCaptureComponent2D)) FilePath FileName))

(fn CreateRenderMaterial
  (bind _asbp_game_mode (Utilities|Casting|CastToBP_GameMode (Game|GetGameMode)))
  (bind _output_get (LocalVariables|SetNewLocalVar (Variables|/Game/Ishikawa/BP_GameMode.BP_GameMode_C|GetRoundSum _asbp_game_mode)))
  (for _index (range 0 (- _output_get 1))
    (bind _returnvalue (Rendering|CreateRenderTarget2D 1024 1024 "RTF_RGBA8"))
    (Utilities|Array|Add (Variables|Default|GetRenderMaterials) _returnvalue)))