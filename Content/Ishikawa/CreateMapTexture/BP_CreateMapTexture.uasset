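; Map texture generator actor that renders an orthographic scene capture of the level and exports the render target to a file.
; It fits to the first BlockingVolume found: centred on its bounds in XY, with height and ortho width of twice the larger horizontal extent.
; This fit runs on construction and again in StartTakeCaptureAndExport, which then captures the scene and writes the file to FilePath and FileName.
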(event Custom|StartTakeCaptureAndExport
  (CallFunction|UpdateSceneCaptureSetting)
  (CallFunction|TakeCapture)
  (CallFunction|ExportSceneTexture (Variables|Default|GetFile%20Path) (Variables|Default|GetFile%20Name)))

(event EventBeginPlay)

(event Collision|EventActorBeginOverlap
  (params (OtherActor :type Actor%20Object%20Reference)))

(event EventTick
  (params (DeltaSeconds :type Float%20%28single-precision%29)))

(fn ConstructionScript
  (CallFunction|UpdateSceneCaptureSetting))

(fn UpdateSceneCaptureSetting
  (bind _returnvalue (Actor|GetActorOfClass "/Script/Engine.BlockingVolume"))
  (Transformation|SetActorLocation (Math|Vector|MakeVector (.x (.Origin (Collision|GetActorBounds _returnvalue false false))) (.y (.Origin (Collision|GetActorBounds _returnvalue false false))) (* (Math|Float|Max(Float) (.x (.BoxExtent (Collision|GetActorBounds _returnvalue false false))) (.y (.BoxExtent (Collision|GetActorBounds _returnvalue false false)))) 2.0)) false false)
  (Class|CameraComponent|SetOrthoWidth (Variables|Default|GetCamera) (* (Math|Float|Max(Float) (.x (.BoxExtent (Collision|GetActorBounds _returnvalue false false))) (.y (.BoxExtent (Collision|GetActorBounds _returnvalue false false)))) 2.0))
  (Development|PrintString (Utilities|String|ToString(Float) (* (Math|Float|Max(Float) (.x (.BoxExtent (Collision|GetActorBounds _returnvalue false false))) (.y (.BoxExtent (Collision|GetActorBounds _returnvalue false false)))) 2.0)))
  (Variables|/Script/Engine.SceneCaptureComponent2D|SetOrthoWidth (Variables|Default|GetSceneCaptureComponent2D) (* (Math|Float|Max(Float) (.x (.BoxExtent (Collision|GetActorBounds _returnvalue false false))) (.y (.BoxExtent (Collision|GetActorBounds _returnvalue false false)))) 2.0)))

(fn TakeCapture
  (Rendering|SceneCapture|CaptureScene (Variables|Default|GetSceneCaptureComponent2D) :!class /Script/Engine.SceneCaptureComponent2D))

(fn ExportSceneTexture
  (params (FilePath :type String) (FileName :type String))
  (Rendering|ExportRenderTarget (Variables|/Script/Engine.SceneCaptureComponent2D|GetTextureTarget (Variables|Default|GetSceneCaptureComponent2D)) FilePath FileName))