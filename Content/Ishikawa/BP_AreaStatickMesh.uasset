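; BP_AreaStatickMesh is a numbered area actor made of static meshes that can be faded out and removed from collision.
; BeginPlay sorts child components into box collisions and meshes, giving each mesh a dynamic material.
; DeleteAreaStart starts a timed ramp of the materials' Threshold parameter on Tick.
; DeleteArea separately adds a nav modifier, sets boxes to query-only and disables mesh collision.
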(event EventBeginPlay
  (for _array_element (Components|GetChildrenComponents (Variables|Default|GetDefaultSceneRoot) true)
    (bind _asbox_collision (Utilities|Casting|CastToBoxComponent _array_element)
      (:then
        (Utilities|Array|Add (Variables|Default|GetBoxCollisions) _asbox_collision))
      (:CastFailed
        (bind _asstatic_mesh_component (Utilities|Casting|CastToStaticMeshComponent _array_element))
        (Utilities|Array|Add (Variables|Default|GetStaticMeshes) _asstatic_mesh_component)
        (bind _returnvalue (Rendering|Material|CreateDynamicMaterialInstance _asstatic_mesh_component 0 (Rendering|Material|GetMaterial _asstatic_mesh_component 0) "None" :!class /Script/Engine.PrimitiveComponent))
        (Utilities|Array|Add (Variables|Default|GetMIDs) _returnvalue)))))

(event Collision|EventActorBeginOverlap
  (params (OtherActor :type Actor%20Object%20Reference)))

(event EventTick
  (params (DeltaSeconds :type Float%20%28single-precision%29))
  (if (Variables|Default|GetIsStartDelete)
    (bind _output_get (Variables|Default|SetDeleteTimeNow (+ DeltaSeconds (Variables|Default|GetDeleteTimeNow))))
    (for _array_element (Variables|Default|GetMIDs)
      (Rendering|Material|SetScalarParameterValue _array_element "Threshold" (/ _output_get (Variables|Default|GetCompleteDeleteSecond)) :!class /Script/Engine.MaterialInstanceDynamic))))

(fn ConstructionScript)

(fn DeleteArea
  (AddComponent|AddNavModifierComponent)
  (for _array_element (Variables|Default|GetBoxCollisions)
    (Collision|SetCollisionEnabled _array_element "QueryOnly"))
  (for _array_element_2 (Variables|Default|GetStaticMeshes)
    (Collision|SetCollisionEnabled _array_element_2 "NoCollision")))

(fn DeleteAreaStart
  (params (CompleteDeleteSecond :type Float%20%28double-precision%29))
  (Variables|Default|SetCompleteDeleteSecond CompleteDeleteSecond)
  (Variables|Default|SetIsStartDelete true)
  (Variables|Default|SetDeleteTimeNow 0.0))

(fn SetAreaNum
  (params (Num :type Integer))
  (Variables|Default|SetAreaNum Num))