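; BP_ObjectActor_storm is a test movable-object actor that carries a Niagara storm effect and is driven by player input.
; BeginPlay spawns the scaled-down effect at SMMoveObject and adds the Enhanced Input mapping; Tick keeps the effect on the mesh.
; The axis action feeds MoveImpact, while the action button only prints debug press and release messages.
; The GetFlip override calls the parent, then disables input and restores it after a short delay.
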(event Custom|DelayInput
  (bind _returnvalue (PlayerController|LocalPlayerSubsystems|GetEnhancedInputLocalPlayerSubsystem 0))
  (Utilities|FlowControl|Delay 0.4)
  (Utilities|FlowControl|Sequence
    (:then_0
      (Input|EnableInput (Variables|Default|GetplayerInput)))
    (:then_1
      (Utilities|IsValid _returnvalue
        (:Is%20Valid
          (Input|AddMappingContext _returnvalue "/Game/kawada/testInput/IMC_Default.IMC_Default" 0 "(bIgnoreAllPressedKeysUntilRelease=True,bForceImmediately=False,bNotifyUserSettings=False)"))))))

(event Input|EnhancedActionEvents|EnhancedInputActionIA_Action
  (params (ActionValue :type Boolean) (ElapsedSeconds :type Float%20%28double-precision%29) (TriggeredSeconds :type Float%20%28double-precision%29) (InputAction :type Input%20Action%20Object%20Reference :default "/Game/kawada/testInput/IA_Action.IA_Action"))
  (:Triggered
    (Utilities|FlowControl|DoOnce false :!label _label
      (:Completed
        (Development|PrintString "Pressed"))))
  (:Completed
    (Utilities|FlowControl|Sequence
      (:then_0
        (goto _label Reset))
      (:then_1
        (Development|PrintString "Released")))))

(event Input|EnhancedActionEvents|EnhancedInputActionIA_Axis
  (params (ActionValue :type Vector%202D%20Structure) (ElapsedSeconds :type Float%20%28double-precision%29) (TriggeredSeconds :type Float%20%28double-precision%29) (InputAction :type Input%20Action%20Object%20Reference :default "/Game/kawada/testInput/IA_Axis.IA_Axis"))
  (bind (_x _y) (Math|Vector2D|BreakVector2D ActionValue))
  (CallFunction|MoveImpact (Math|Vector|MakeVector _x _y 0.0)))

(event EventBeginPlay
  (bind _returnvalue (Game|GetPlayerController 0))
  (bind _returnvalue_2 (PlayerController|LocalPlayerSubsystems|GetEnhancedInputLocalPlayerSubsystem _returnvalue))
  (|CallParentFunction)
  (bind _returnvalue_3 (Niagara|SpawnSystematLocation "/Game/shirota/NA_Storm2.NA_Storm2" (Transformation|GetWorldLocation (Variables|Default|GetSM_moveObject)) "0, 0, 0" "0.200000,0.200000,0.200000"))
  (Variables|Default|SetNiagara_0 _returnvalue_3)
  (Utilities|FlowControl|Sequence
    (:then_0
      (bind _output_get (Variables|Default|SetplayerInput _returnvalue))
      (Input|EnableInput _output_get))
    (:then_1
      (Utilities|IsValid _returnvalue_2
        (:Is%20Valid
          (Input|AddMappingContext _returnvalue_2 "/Game/kawada/testInput/IMC_Default.IMC_Default" 0 "(bIgnoreAllPressedKeysUntilRelease=True,bForceImmediately=False,bNotifyUserSettings=False)"))))))

(event Collision|EventActorBeginOverlap
  (params (OtherActor :type Actor%20Object%20Reference))
  (|CallParentFunction OtherActor) ; このノードは無効になっているため呼び出せません。\n機能をビルドするにはピンをドラッグしてください。
)

(event EventTick
  (params (DeltaSeconds :type Float%20%28single-precision%29))
  (Transformation|SetWorldLocation (Variables|Default|GetNiagara_0) (Transformation|GetWorldLocation (Variables|Default|GetSM_moveObject)) false false))

(fn ConstructionScript
  (|CallParentFunction))

(fn GetFlip
  (|CallParentFunction)
  (Input|DisableInput (Variables|Default|GetplayerInput))
  (CallFunction|DelayInput))