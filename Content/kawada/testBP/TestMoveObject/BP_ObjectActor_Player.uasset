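; Player-controlled child of an object actor base, driven by Enhanced Input for impulse-style movement and a once-per-press dash.
; Game mode events disable input at start, then re-enable it and create the HUD at game start.
; Tick feeds normalized speed to the HUD, while Damage and Heal overrides update its HP display.
; CheckHitStop triggers time-dilation hit stop above a speed threshold, plus a timeline-driven spring-arm camera effect.
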(event Custom|CameraDirection
  ;[1 1 1] ヒットストップ時のカメラワーク
  (Variables|一時保存用|SetarmLength (Variables|/Script/Engine.SpringArmComponent|GetTargetArmLength (Variables|Default|GetSpringArm_0)))
  (bind _新規track_0 (Timeline|Cam PlayFromStart)
    (:Update
      (Variables|/Script/Engine.SpringArmComponent|SetTargetArmLength (Variables|Default|GetSpringArm_0) (+ (* _新規track_0 (Variables|Default|GetArmDistance)) (Variables|一時保存用|GetarmLength))))))

(event Custom|Dis%20input
  ;[1 1 1] イベントの登録
  (Input|DisableInput (Game|GetPlayerController 0)))

(event Custom|Ena%20Input
  ;[1 1 1] イベントの登録
  (Development|PrintString "操作可能" true true "(R=0.010387,G=1.000000,B=0.000000,A=1.000000)")
  (Input|EnableInput (Game|GetPlayerController 0))
  ;[1 1 1] UIの設定と初期化
  (bind _returnvalue (Game|ConstructObjectfromClass "/Game/kawada/WIdget/WBP_GameUI.WBP_GameUI_C"))
  (bind _output_get (Variables|一時保存用|SetGameUI _returnvalue))
  (UserInterface|Viewport|AddtoViewport _output_get 0)
  (Variables|/Game/kawada/WIdget/WBP_GameUI.WBP_GameUI_C|SetDrawHP _output_get 1.0))

(event Input|EnhancedActionEvents|EnhancedInputActionIA_Action
  (params (ActionValue :type Boolean) (ElapsedSeconds :type Float%20%28double-precision%29) (TriggeredSeconds :type Float%20%28double-precision%29) (InputAction :type Input%20Action%20Object%20Reference :default "/Game/kawada/testInput/IA_Action.IA_Action"))
  ;[1 1 1] ボタンの取得とダッシュ
  (:Triggered
    (Utilities|FlowControl|DoOnce false :!label _label
      (:Completed
        (Development|PrintString "Pressed")
        (CallFunction|Dash))))
  (:Completed
    (Utilities|FlowControl|Sequence
      (:then_0
        (goto _label Reset))
      (:then_1
        (Development|PrintString "Released")))))

(event Input|EnhancedActionEvents|EnhancedInputActionIA_Axis
  (params (ActionValue :type Vector%202D%20Structure) (ElapsedSeconds :type Float%20%28double-precision%29) (TriggeredSeconds :type Float%20%28double-precision%29) (InputAction :type Input%20Action%20Object%20Reference :default "/Game/kawada/testInput/IA_Axis.IA_Axis"))
  (bind (_x _y) (Math|Vector2D|BreakVector2D ActionValue))
  ;[1 1 1] 移動
  (CallFunction|MoveImpact (Math|Vector|MakeVector _x _y 0.0)))

(event EventBeginPlay
  (bind _returnvalue (Game|GetPlayerController 0))
  (bind _returnvalue_2 (PlayerController|LocalPlayerSubsystems|GetEnhancedInputLocalPlayerSubsystem _returnvalue))
  ;[1 1 1] 親クラスの初期化処理から
  (|CallParentFunction)
  (Variables|Default|SetFaceMat (Variables|Default|GetFace%20Mat))
  ;[1 1 1] コントローラーの初期化
  (Utilities|FlowControl|Sequence
    (:then_0
      (bind _output_get (Variables|Default|SetplayerInput _returnvalue))
      (Input|EnableInput _output_get)
      ;[1 1 1] イベントの登録
      (bind _asbp_game_mode (Utilities|Casting|CastToBP_GameMode (Game|GetGameMode)))
      (EventDispatchers|BindEventtoStart _asbp_game_mode (delegate Custom|Dis%20input))
      (EventDispatchers|BindEventtoGameStart _asbp_game_mode (delegate Custom|Ena%20Input)))
    (:then_1
      (Utilities|IsValid _returnvalue_2
        (:Is%20Valid
          (Input|AddMappingContext _returnvalue_2 "/Game/kawada/testInput/IMC_Default.IMC_Default" 0 "(bIgnoreAllPressedKeysUntilRelease=True,bForceImmediately=False,bNotifyUserSettings=False)"))))))

(event EventTick
  (params (DeltaSeconds :type Float%20%28single-precision%29))
  (bind _gameui (Variables|一時保存用|GetGameUI))
  (bind _floatingpawnmovement (Variables|Default|GetFloatingPawnMovement))
  ;[1 1 1] 速度UIの設定
  (|CallParentFunction DeltaSeconds)
  (Utilities|IsValid _gameui
    (:Is%20Valid
      (Variables|/Game/kawada/WIdget/WBP_GameUI.WBP_GameUI_C|SetSpeed _gameui (/ (Math|Vector|VectorLength (Variables|/Script/Engine.MovementComponent|GetVelocity _floatingpawnmovement)) (Class|MovementComponent|GetMaxSpeed _floatingpawnmovement))))))

(fn ConstructionScript
  (|CallParentFunction))

(fn Dead
  (Input|EnableInput (Variables|Default|GetplayerInput))
  (|CallParentFunction))

(fn CheckHitStop
  (bind _floatingpawnmovement (Variables|Default|GetFloatingPawnMovement))
  (if (>= (Math|Vector|VectorLength (Variables|/Script/Engine.MovementComponent|GetVelocity _floatingpawnmovement)) (* (Variables|/Script/Engine.FloatingPawnMovement|GetMaxSpeed _floatingpawnmovement) (/ (Variables|Default|GetHitstopThreshold) 100)))
    (CallFunction|HitStop 0.025 (Variables|Default|GethitStopTime))
    (Utilities|Time|SetTimerbyFunctionName 0 "CameraDirection" 0.01)))

(fn Damage
  (params (inDamage :type Integer))
  (bind _gameui (Variables|一時保存用|GetGameUI))
  (|CallParentFunction inDamage)
  (Utilities|IsValid _gameui
    (:Is%20Valid
      (Default|UIDamage _gameui (/ (Math|Conversions|ToFloat(Integer) (Variables|Default|GetHP)) (.maxhp (Variables|Default|GetsuperficialStatus)))))))

(fn Heal
  (params (inHeal :type Integer))
  (bind _gameui (Variables|一時保存用|GetGameUI))
  (bind _isover (|CallParentFunction inHeal))
  (Utilities|IsValid _gameui
    (:Is%20Valid
      (Variables|/Game/kawada/WIdget/WBP_GameUI.WBP_GameUI_C|SetDrawHP _gameui (/ (Math|Conversions|ToFloat(Integer) (Variables|Default|GetHP)) (.maxhp (Variables|Default|GetsuperficialStatus)))))
    (:Is%20Not%20Valid
      _))
  (return _isover))