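; Test battle pawn with spinning item mounts that moves by input and knocks other BP_ObjectActors away on overlap.
; Collisions compare speed times spin to scale damage and impulse, with hit stop for max-speed winners, invulnerability, input lockout and knockback distance tracking.
; 0–100-style stats map to internal ranges, driving movement, HP, delayed regen and an HP-cost dash.
; Each tick, a ring of ray traces records drop directions for missing ground.
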(event OnComponentBeginOverlap(InColl)
  (params (OverlappedComponent :type Primitive%20Component%20Object%20Reference) (OtherActor :type Actor%20Object%20Reference) (OtherComp :type Primitive%20Component%20Object%20Reference) (OtherBodyIndex :type Integer) (bFromSweep :type Boolean) (SweepResult :type Hit%20Result%20Structure%20%28by%20ref%29))
  (bind _powervalue (Variables|ローカルステータス|GetpowerValue))
  (bind _floatingpawnmovement (Variables|Default|GetFloatingPawnMovement))
  (bind _floatingpawnmovement_2 (Variables|Default|GetFloatingPawnMovement))
  (bind _flipstatus (Variables|ステータス管理用|GetflipStatus))
  ;[1 1 1] 弾く仮実装
  (if (not (Variables|可否|GetisHit))
    (if (!= OtherComp (Variables|Default|GetInColl))
      (bind _asbp_object_actor (Utilities|Casting|CastToBP_ObjectActor OtherActor))
      (Utilities|Casting|CastToCapsuleComponent OtherComp)
      (if (Variables|可否|GetisOperation)
        _
        (else
          (アクション|SendFlipDistance)
          (Utilities|Time|ClearandInvalidateTimerbyHandle (Variables|ローカル|GetInoperable_Handle))))
      (Variables|ローカル|SethitActorLocation (Transformation|GetActorLocation _asbp_object_actor))
      (bind _output_get (Variables|ローカル|SethitActor _asbp_object_actor))
      (bind _multires (取得|GetCompStatus _output_get))
      (bind (_speed _rotspeed _multires_2 _vector) (取得|GetCompStatus))
      (if (>= _multires_2 _multires)
        ;;[1 1 1] ステータスで勝っていた場合
        (Variables|ローカル|Set_damage (Math|Float|Round (/ (* (Math|Float|Lerp (.low _powervalue) (.high _powervalue) (Math|Float|Clamp(Float) (/ (- _multires_2 _multires) (.flipdisstatus _flipstatus)))) (* (+ (Math|Vector|VectorLength _vector) 1.0) (Math|Float|Lerp 0.8 1.5 (/ (+ (Math|Vector|DotProduct (Math|Vector|Normalize (Math|Vector|GetUnitDirection(Vector) (Transformation|GetActorLocation) (Transformation|GetActorLocation _asbp_object_actor))) (Transformation|GetActorForwardVector (Variables|ローカル|GethitActor))) 1.0) 2.0)))) (Math|Float|Lerp 1.0 1e+03 (/ (Math|Vector|VectorLength (Variables|/Script/Engine.MovementComponent|GetVelocity _floatingpawnmovement_2)) (Class|MovementComponent|GetMaxSpeed _floatingpawnmovement_2))))))
        (アクション|ImpulseAction (Variables|ローカル|GethitActor) (* (Math|Vector|GetUnitDirection(Vector) (Transformation|GetActorLocation) (Transformation|GetActorLocation _asbp_object_actor)) (+ (Math|Float|Lerp (.lowflippow _flipstatus) (.highflippow _flipstatus) (Math|Float|Clamp(Float) (/ (- _multires_2 _multires) (.flipdisstatus _flipstatus)))) (* (+ (Math|Vector|VectorLength _vector) 1.0) (Math|Float|Lerp 0.8 1.5 (/ (+ (Math|Vector|DotProduct (Math|Vector|Normalize (Math|Vector|GetUnitDirection(Vector) (Transformation|GetActorLocation) (Transformation|GetActorLocation _asbp_object_actor))) (Transformation|GetActorForwardVector (Variables|ローカル|GethitActor))) 1.0) 2.0))))))
        (Variables|可否|SetisWin true)
        ;;[1 1 1] 最大速度ならヒットストップ
        (if (>= (Math|Vector|VectorLength (Variables|/Script/Engine.MovementComponent|GetVelocity _floatingpawnmovement)) (Variables|/Script/Engine.FloatingPawnMovement|GetMaxSpeed _floatingpawnmovement))
          (CallFunction|HitStop 0.025 1.0))
        (else
          ;;[1 1 1] ステータスで負けていた場合
          (Variables|ローカル|Set_damage (Math|Float|Round (* (/ (* (Math|Float|Lerp (.low _powervalue) (.high _powervalue) (Math|Float|Clamp(Float) (/ (- _multires_2 _multires) (.flipdisstatus _flipstatus)))) (* (+ (Math|Vector|VectorLength _vector) 1.0) (Math|Float|Lerp 0.8 1.5 (/ (+ (Math|Vector|DotProduct (Math|Vector|Normalize (Math|Vector|GetUnitDirection(Vector) (Transformation|GetActorLocation) (Transformation|GetActorLocation _asbp_object_actor))) (Transformation|GetActorForwardVector (Variables|ローカル|GethitActor))) 1.0) 2.0)))) (Math|Float|Lerp 1.0 1e+03 (/ (Math|Vector|VectorLength (Variables|/Script/Engine.MovementComponent|GetVelocity _floatingpawnmovement_2)) (Class|MovementComponent|GetMaxSpeed _floatingpawnmovement_2)))) 0.2)))
          (アクション|ImpulseAction (Variables|ローカル|GethitActor) (* (Math|Vector|GetUnitDirection(Vector) (Transformation|GetActorLocation) (Transformation|GetActorLocation _asbp_object_actor)) (* (+ (Math|Float|Lerp (.lowflippow _flipstatus) (.highflippow _flipstatus) (Math|Float|Clamp(Float) (/ (- _multires_2 _multires) (.flipdisstatus _flipstatus)))) (* (+ (Math|Vector|VectorLength _vector) 1.0) (Math|Float|Lerp 0.8 1.5 (/ (+ (Math|Vector|DotProduct (Math|Vector|Normalize (Math|Vector|GetUnitDirection(Vector) (Transformation|GetActorLocation) (Transformation|GetActorLocation _asbp_object_actor))) (Transformation|GetActorForwardVector (Variables|ローカル|GethitActor))) 1.0) 2.0)))) 0.2)))
          (Variables|可否|SetisWin false)))
      (アクション|Damage (Variables|ローカル|GethitActor) (Variables|ローカル|Get_damage))
      (取得|GetFlip)
      (if (Variables|デバッグ用|GetDebugHit)
        (Development|PrintString (Utilities|String|Append (Utilities|GetDisplayName (Variables|ローカル|GethitActor)) " ： " (Utilities|String|ToString(Integer) (Variables|ローカル|Get_damage))) true true "(R=0.000000,G=0.660000,B=1.000000,A=1.000000)" 5.0))
      ;;[1 1 1] 無敵時間の時間設定
      (Utilities|Time|SetTimerbyFunctionName 0 "DownTime" (Variables|初期値|GetInvDownTime))
      ;;[1 1 1] 吹っ飛ばされた距離の計測開始
      (bind _returnvalue (Utilities|Time|SetTimerbyFunctionName 0 "Inoperable" (Variables|初期値|GetInoperableTime)))
      (Variables|ローカル|SetInoperable_Handle _returnvalue) ; 計測中に新規で吹っ飛ばされた時用
    )))

(event Custom|HitStop
  (params (inTimeDilation :type Float%20%28double-precision%29) (inDuration :type Float%20%28double-precision%29))
  ;[1 1 1] ヒットストップ
  (Utilities|Time|SetGlobalTimeDilation inTimeDilation)
  (Utilities|FlowControl|Delay (* inTimeDilation inDuration))
  (Utilities|Time|SetGlobalTimeDilation 1.0))

(event Custom|DownTime
  ;[1 1 1] 無敵時間
  (Variables|可否|SetisHit false)
  (Development|PrintString "無敵時間終了" true true "(R=1.000000,G=0.065980,B=0.000000,A=1.000000)"))

(event Custom|MoveImpact
  (params (ImpactParam :type Vector))
  (bind _returnvalue (Transformation|GetActorLocation))
  (bind _floatingpawnmovement (Variables|Default|GetFloatingPawnMovement))
  (bind _sm_moveobject (Variables|Default|GetSM_moveObject))
  (bind _returnvalue_2 (Transformation|GetWorldLocation _sm_moveobject))
  ;[1 1 1] 移動関数
  (if (Variables|可否|GetisOperation)
    (Class|PawnMovementComponent|AddInputVector _floatingpawnmovement ImpactParam false)
    (Rendering|Debug|DrawDebugArrow _returnvalue_2 (+ _returnvalue_2 (Variables|/Script/Engine.MovementComponent|GetVelocity _floatingpawnmovement)) 2.0 "(R=0.000000,G=0.043990,B=1.000000,A=1.000000)" 0.0 0.0)
    ;[1 1 1] 回転
    (if (< 0.0 (Math|Vector|VectorLength ImpactParam))
      (Transformation|SetActorRotation (Math|Interpolation|RInterpTo (Transformation|GetActorRotation) (Math|Rotator|FindLookatRotation _returnvalue (+ _returnvalue (* 1e+02 ImpactParam))) (Utilities|Time|GetWorldDeltaSeconds) 6.0)))))

(event Custom|Inoperable
  ;[1 1 1] 操作不能
  (アクション|SendFlipDistance)
  (if (not (Variables|可否|GetisDead))
    (Variables|可否|SetisOperation true)))

(event Custom|WakeUpRegen
  ;[1 1 1] リジェネの起動
  (if (not (Variables|可否|GetisDead))
    (Utilities|Time|SetTimerbyFunctionName 0 "Regen" (.regenraito (Variables|ステータス|GetregenStatus)) true)
    (Variables|ステータス|SetregenStatus (Utilities|Struct|MakeRegenStatus true (.sregentime (Variables|ステータス|GetregenStatus)) (.regenraito (Variables|ステータス|GetregenStatus))))
    (Development|PrintString "リジェネの起動")))

(event Custom|Regen
  (bind _regenvalue (Variables|ローカルステータス|GetregenValue))
  (bind _returnvalue (Math|Float|Truncate _regenvalue))
  ;[1 1 1] リジェネ
  (if (.isregen (Variables|ステータス|GetregenStatus))
    (if (> _returnvalue 0)
      (bind _isover (アクション|Heal _returnvalue))
      (Development|PrintString (Utilities|String|Append "Regen : " (Utilities|String|ToString(Integer) _returnvalue)))
      (if _isover
        (Utilities|Time|ClearTimerbyFunctionName 0 "Regen")
        (Development|PrintString "自動回復終了" true true "(R=1.000000,G=0.005320,B=0.000000,A=1.000000)")))))

(event Custom|dashEnd
  ;[1 1 1] ダッシュの終了処理
  (設定|SetStatus "NewEnumerator2" (Variables|ローカル|GetdefAcc))
  (設定|SetStatus "NewEnumerator1" (Variables|ローカル|GetdefMaxSpeed))
  (Variables|ステータス|SetdashStatus (Utilities|Struct|MakeDashStatus false (.dashtime (Variables|ステータス|GetdashStatus)) (.dashspeed (Variables|ステータス|GetdashStatus)) (.hpcost (Variables|ステータス|GetdashStatus))))
  (Development|PrintString "高速移動終了" true true "(R=1.000000,G=0.080961,B=0.000000,A=1.000000)"))

(event EventBeginPlay
  ;[1 1 1] 初期化
  (if (Variables|初期値|GetisDefaultStatus)
    (bind _asbp_level_mg (Utilities|Casting|CastToBP_LevelMG (Game|GetGameInstance))
      (:then
        (bind _defaultstatus (Default|GetDefaultEnemyStatus _asbp_level_mg))
        (Variables|ステータス管理用|SetflipStatus _defaultstatus))
      (:CastFailed
        _)))
  (設定|InitStatus (Variables|ステータス|GetsuperficialStatus)))

(event EventTick
  (params (DeltaSeconds :type Float%20%28single-precision%29))
  (bind _returnvalue (Transformation|GetActorLocation))
  (bind _items (Variables|Default|GetItems))
  ;[1 1 1] 正面方向ベクトルの表示
  (if (not (Variables|可否|GetisDead))
    (Rendering|Debug|DrawDebugArrow _returnvalue (+ _returnvalue (* (Transformation|GetActorForwardVector) 1e+02)) 1.0 "(R=1.000000,G=0.000000,B=0.941127,A=1.000000)" 0.0 0.0)
    (Transformation|SetWorldRotation _items (Math|Rotator|CombineRotators (Transformation|GetWorldRotation _items) (Math|Rotator|MakeRotator 0.0 0.0 (Variables|ローカルステータス|GetRotSpeed))) false false)
    (取得|CalcRay)
    (|ItemPointDraw)))

(event EventParticleData
  (params (Data :type Array%20of%20Basic%20Particle%20Data%20Structures) (NiagaraSystem :type Niagara%20System%20Object%20Reference) (SimulationPositionOffset :type Vector%20%28by%20ref%29 :default "0, 0, 0"))
  ;[1 1 1] Niagara用
)

(fn ConstructionScript)

(fn ImpulseAction
  (params (PalseValue :type Vector))
  (Physics|AddImpulse (Variables|Default|GetSM_moveObject) PalseValue "None" true))

(fn GetFlip
  (Variables|可否|SetisHit true)
  (Variables|可否|SetisOperation false))

(fn GetCompStatus
  (bind _rotspeed (Variables|ローカルステータス|GetRotSpeed))
  (bind _floatingpawnmovement (Variables|Default|GetFloatingPawnMovement))
  (bind _superficialstatus (Variables|ステータス|GetsuperficialStatus))
  (bind _returnvalue (/ (.maxspeed _superficialstatus) 100))
  (bind _velocity (Variables|/Script/Engine.MovementComponent|GetVelocity _floatingpawnmovement))
  (bind _ret (取得|GetOneStatusforFloat "NewEnumerator1" _returnvalue))
  (bind _returnvalue_2 (Math|Vector|VectorLength _velocity))
  (bind _returnvalue_3 (+ _returnvalue_2 1.0))
  (bind _returnvalue_4 (/ _returnvalue_3 _ret))
  (return _returnvalue_4 _rotspeed (* _returnvalue_4 _rotspeed) _velocity))

(fn SetStatus
  (params (inName :type StatusName%20Enum :default "NewEnumerator0") (inValue :type Integer))
  (switch Utilities|FlowControl|Switch|SwitchonStatusName inName
    (:NewEnumerator0
      (bind _output_get (Variables|ステータス|SetsuperficialStatus (Utilities|Struct|MakeSuperficialStatus inValue (.maxspeed (Variables|ステータス|GetsuperficialStatus)) (.acceleration (Variables|ステータス|GetsuperficialStatus)) (.maxhp (Variables|ステータス|GetsuperficialStatus)) (.resilience (Variables|ステータス|GetsuperficialStatus)))))
      (Variables|ローカルステータス|SetpowerValue (Utilities|Struct|MakeHighLowFloat (.low (Variables|ローカルステータス|GetpowerValue)) (取得|GetOneStatusforInt "NewEnumerator0" (.power _output_get)))))
    (:NewEnumerator1
      (bind _output_get_2 (Variables|ステータス|SetsuperficialStatus (Utilities|Struct|MakeSuperficialStatus (.power (Variables|ステータス|GetsuperficialStatus)) inValue (.acceleration (Variables|ステータス|GetsuperficialStatus)) (.maxhp (Variables|ステータス|GetsuperficialStatus)) (.resilience (Variables|ステータス|GetsuperficialStatus)))))
      (Variables|/Script/Engine.FloatingPawnMovement|SetMaxSpeed (Variables|Default|GetFloatingPawnMovement) (取得|GetOneStatusforInt "NewEnumerator1" (.maxspeed _output_get_2))))
    (:NewEnumerator2
      (bind _output_get_3 (Variables|ステータス|SetsuperficialStatus (Utilities|Struct|MakeSuperficialStatus (.power (Variables|ステータス|GetsuperficialStatus)) (.maxspeed (Variables|ステータス|GetsuperficialStatus)) inValue (.maxhp (Variables|ステータス|GetsuperficialStatus)) (.resilience (Variables|ステータス|GetsuperficialStatus)))))
      (Variables|/Script/Engine.FloatingPawnMovement|SetAcceleration (Variables|Default|GetFloatingPawnMovement) (取得|GetOneStatusforInt "NewEnumerator2" (.acceleration _output_get_3))))
    (:NewEnumerator3
      (Variables|ステータス|SetsuperficialStatus (Utilities|Struct|MakeSuperficialStatus (.power (Variables|ステータス|GetsuperficialStatus)) (.maxspeed (Variables|ステータス|GetsuperficialStatus)) (.acceleration (Variables|ステータス|GetsuperficialStatus)) inValue (.resilience (Variables|ステータス|GetsuperficialStatus))))
      (アクション|Heal (Math|Float|Truncate (- (取得|GetOneStatusforInt "NewEnumerator3" (.maxhp (Variables|ステータス|GetsuperficialStatus))) (取得|GetOneStatusforInt "NewEnumerator3" inValue)))))
    (:NewEnumerator4
      (bind _output_get_4 (Variables|ステータス|SetsuperficialStatus (Utilities|Struct|MakeSuperficialStatus (.power (Variables|ステータス|GetsuperficialStatus)) (.maxspeed (Variables|ステータス|GetsuperficialStatus)) (.acceleration (Variables|ステータス|GetsuperficialStatus)) (.maxhp (Variables|ステータス|GetsuperficialStatus)) inValue)))
      (Variables|ローカルステータス|SetregenValue (取得|GetOneStatusforInt "NewEnumerator4" (.resilience _output_get_4))))))

(fn GetIsHit
  (return (Variables|可否|GetisHit)))

(fn Damage
  (params (inDamage :type Integer))
  (bind _output_get (Variables|ローカルステータス|SetHP (- (Variables|ローカルステータス|GetHP) inDamage)))
  (Variables|ステータス|SetregenStatus (Utilities|Struct|MakeRegenStatus false (.sregentime (Variables|ステータス|GetregenStatus)) (.regenraito (Variables|ステータス|GetregenStatus))))
  (Utilities|Time|SetTimerbyFunctionName 0 "WakeUpRegen" (.sregentime (Variables|ステータス|GetregenStatus)))
  (Development|PrintString (Utilities|String|Append " HP ：" (Utilities|String|ToString(Integer) _output_get)))
  (if (<= (Variables|ローカルステータス|GetHP) 0)
    (アクション|Dead)))

(fn Heal
  (params (inHeal :type Integer))
  (bind _superficialstatus (Variables|ステータス|GetsuperficialStatus))
  (if (not (< (+ inHeal (Variables|ローカルステータス|GetHP)) (.maxhp _superficialstatus)))
    (Variables|ローカルステータス|SetHP (.maxhp _superficialstatus))
    (return true)
    (else
      (Variables|ローカルステータス|SetHP (+ inHeal (Variables|ローカルステータス|GetHP)))
      (return false))))

(fn AddBlowDistance
  (params (NewParam :type Float%20%28double-precision%29))
  (Variables|ステータス管理用|SetresultStatus (Utilities|Struct|MakeGameResultStatus (.rank (Variables|ステータス管理用|GetresultStatus)) (+ NewParam (.flydis (Variables|ステータス管理用|GetresultStatus))) (.enflydis (Variables|ステータス管理用|GetresultStatus)) (.itennum (Variables|ステータス管理用|GetresultStatus)))))

(fn AddItems
  (Variables|ステータス管理用|SetresultStatus (Utilities|Struct|MakeGameResultStatus (.rank (Variables|ステータス管理用|GetresultStatus)) (.flydis (Variables|ステータス管理用|GetresultStatus)) (.enflydis (Variables|ステータス管理用|GetresultStatus)) (+ (.itennum (Variables|ステータス管理用|GetresultStatus)) 1))))

(fn GetResultStatus
  (return (Variables|ステータス管理用|GetresultStatus)))

(fn SendFlipDistance
  (bind _returnvalue (Transformation|GetActorLocation))
  (bind _hitactor (Variables|ローカル|GethitActor))
  (bind _hitactorlocation (Variables|ローカル|GethitActorLocation))
  (bind _returnvalue_2 (Math|Vector|Distance(Vector) _hitactorlocation _returnvalue))
  (bind _returnvalue_3 (Math|Float|Absolute(Float) _returnvalue_2))
  (Utilities|IsValid _hitactor
    (:Is%20Valid
      (計算|AddBlowDistance _hitactor _returnvalue_3)
      ;[1 1 1] 自身の変数に吹っ飛ばされた距離の加算
      (Variables|ステータス管理用|SetresultStatus (Utilities|Struct|MakeGameResultStatus (.rank (Variables|ステータス管理用|GetresultStatus)) (.flydis (Variables|ステータス管理用|GetresultStatus)) (+ (.enflydis (Variables|ステータス管理用|GetresultStatus)) _returnvalue_3) (.itennum (Variables|ステータス管理用|GetresultStatus)))))))

(fn Dash
  (bind _superficialstatus (Variables|ステータス|GetsuperficialStatus))
  (if (not (.dashfrag (Variables|ステータス|GetdashStatus)))
    (if (> (- (Variables|ローカルステータス|GetHP) (Math|Float|Truncate (* (/ (.hpcost (Variables|ステータス|GetdashStatus)) 1e+02) (.maxhp (Variables|ステータス|GetsuperficialStatus))))) 0)
      (Development|PrintString "高速移動開始" true true "(R=0.000000,G=1.000000,B=0.104723,A=1.000000)")
      (Variables|ステータス|SetdashStatus (Utilities|Struct|MakeDashStatus true (.dashtime (Variables|ステータス|GetdashStatus)) (.dashspeed (Variables|ステータス|GetdashStatus)) (.hpcost (Variables|ステータス|GetdashStatus))))
      (アクション|Damage (Math|Float|Truncate (* (/ (.hpcost (Variables|ステータス|GetdashStatus)) 1e+02) (.maxhp (Variables|ステータス|GetsuperficialStatus)))))
      (Variables|ローカル|SetdefMaxSpeed (.maxspeed _superficialstatus))
      (Variables|ローカル|SetdefAcc (.acceleration _superficialstatus))
      (設定|SetStatus "NewEnumerator2" 100)
      (設定|SetStatus "NewEnumerator1" 100)
      (Utilities|Time|SetTimerbyFunctionName 0 "dashEnd" (.dashtime (Variables|ステータス|GetdashStatus)))
      (else
        (Development|PrintString "体力が足りません" true true "(R=1.000000,G=0.040184,B=0.000000,A=1.000000)")))))

(fn Dead
  (Development|PrintString "Dead" true true "(R=1.000000,G=0.031556,B=0.000000,A=1.000000)")
  (Variables|可否|SetisDead true)
  (Rendering|SetVisibility (Variables|Default|GetSM_moveObject) false true)
  (Collision|SetCollisionEnabled (Variables|Default|GetInColl) "NoCollision"))

(fn GetOneStatusforInt
  (params (inName :type StatusName%20Enum :default "NewEnumerator0") (inValue :type Integer))
  (bind _internalstatus (Variables|ステータス管理用|GetinternalStatus))
  (switch Utilities|FlowControl|Switch|SwitchonStatusName inName
    (:NewEnumerator0
      (return (Math|Float|Lerp (.low (.power _internalstatus)) (.high (.power _internalstatus)) (/ inValue 100))))
    (:NewEnumerator1
      (return (Math|Float|Lerp (.low (.maxspeed _internalstatus)) (.high (.maxspeed _internalstatus)) (/ inValue 100))))
    (:NewEnumerator2
      (return (Math|Float|Lerp (.low (.acceleration _internalstatus)) (.high (.acceleration _internalstatus)) (/ inValue 100))))
    (:NewEnumerator3
      (return (Math|Float|Lerp (.low (.hitpoints _internalstatus)) (.high (.hitpoints _internalstatus)) (/ inValue 10000))))
    (:NewEnumerator4
      (return (Math|Float|Lerp (.low (.resilience _internalstatus)) (.high (.resilience _internalstatus)) (/ inValue 500))))))

(fn GetOneStatusforFloat
  (params (inName :type StatusName%20Enum :default "NewEnumerator0") (inValue :type Float%20%28double-precision%29))
  (bind _internalstatus (Variables|ステータス管理用|GetinternalStatus))
  (switch Utilities|FlowControl|Switch|SwitchonStatusName inName
    (:NewEnumerator0
      (return (Math|Float|Lerp (.low (.power _internalstatus)) (.high (.power _internalstatus)) inValue)))
    (:NewEnumerator1
      (return (Math|Float|Lerp (.low (.maxspeed _internalstatus)) (.high (.maxspeed _internalstatus)) inValue)))
    (:NewEnumerator2
      (return (Math|Float|Lerp (.low (.acceleration _internalstatus)) (.high (.acceleration _internalstatus)) inValue)))
    (:NewEnumerator3
      (return (Math|Float|Lerp (.low (.hitpoints _internalstatus)) (.high (.hitpoints _internalstatus)) inValue)))
    (:NewEnumerator4
      (return (Math|Float|Lerp (.low (.resilience _internalstatus)) (.high (.resilience _internalstatus)) inValue)))))

(fn CalcRay
  (bind _sm_moveobject (Variables|Default|GetSM_moveObject))
  (bind _sm_moveobject_2 (Variables|Default|GetSM_moveObject))
  (bind _returnvalue (Transformation|GetWorldLocation _sm_moveobject))
  (bind _returnvalue_2 (Transformation|GetWorldLocation _sm_moveobject))
  (bind _returnvalue_3 (+ (.z _returnvalue) 1.2e+02))
  (bind _returnvalue_4 (Math|Vector|MakeVector (.x _returnvalue) (.y _returnvalue) _returnvalue_3))
  (for _index (range 0 9)
    (bind _returnvalue_5 (Collision|LineTraceForObjects _returnvalue_4 (+ _returnvalue_4 (Math|Vector|RotateVectorAroundAxis (Math|Vector|RotateVectorAroundAxis (- (Math|Vector|MakeVector (.x _returnvalue_2) (.y _returnvalue_2) (- (.z _returnvalue_2) 1e+03)) _returnvalue_4) 78.0 (Math|Vector|GetForwardVector _sm_moveobject_2)) (* _index 36) (Math|Vector|GetUpVector _sm_moveobject_2))) (Utilities|Array|MakeArray "ObjectTypeQuery1") false 0 "ForOneFrame"))
    (if (not _returnvalue_5)
      (Utilities|Array|Add (Variables|Default|GetDropVector) (Math|Vector|Normalize (- (+ _returnvalue_4 (Math|Vector|RotateVectorAroundAxis (Math|Vector|RotateVectorAroundAxis (- (Math|Vector|MakeVector (.x _returnvalue_2) (.y _returnvalue_2) (- (.z _returnvalue_2) 1e+03)) _returnvalue_4) 78.0 (Math|Vector|GetForwardVector _sm_moveobject_2)) (* _index 36) (Math|Vector|GetUpVector _sm_moveobject_2))) (Transformation|GetWorldLocation (Variables|Default|GetSM_moveObject))))))))

(fn InitStatus
  (params (inValue :type Superficial%20Status%20Structure))
  (設定|SetStatus "NewEnumerator0" (.power inValue))
  (設定|SetStatus "NewEnumerator1" (.maxspeed inValue))
  (設定|SetStatus "NewEnumerator2" (.acceleration inValue))
  (設定|SetStatus "NewEnumerator3" (.maxhp inValue))
  (設定|SetStatus "NewEnumerator4" (.resilience inValue))
  (Variables|ローカルステータス|SetHP (.maxhp inValue)))

(fn GetStatus
  (bind _floatingpawnmovement (Variables|Default|GetFloatingPawnMovement))
  (return (.high (Variables|ローカルステータス|GetpowerValue)) (Variables|/Script/Engine.FloatingPawnMovement|GetAcceleration _floatingpawnmovement) (Class|MovementComponent|GetMaxSpeed _floatingpawnmovement) (Variables|ローカルステータス|GetHP) (Variables|ローカルステータス|GetregenValue)))

(fn AddStatus
  (params (serectName :type StatusName%20Enum :default "NewEnumerator0") (inValue :type Integer))
  (bind _superficialstatus (Variables|ステータス|GetsuperficialStatus))
  (switch Utilities|FlowControl|Switch|SwitchonStatusName serectName
    (:NewEnumerator0
      ;[1 1 1] Powerの加算
      (設定|SetStatus "NewEnumerator0" (Math|Integer|Clamp(Integer) (+ (.power _superficialstatus) inValue) 0 100)))
    (:NewEnumerator1
      ;[1 1 1] MaxSpeedの加算
      (設定|SetStatus "NewEnumerator1" (Math|Integer|Clamp(Integer) (+ (.maxspeed _superficialstatus) inValue) 0 100)))
    (:NewEnumerator2
      ;[1 1 1] Accelerationの加算
      (設定|SetStatus "NewEnumerator2" (Math|Integer|Clamp(Integer) (+ (.acceleration _superficialstatus) inValue) 0 100)))
    (:NewEnumerator3
      ;[1 1 1] HPの加算
      (設定|SetStatus "NewEnumerator3" (Math|Integer|Clamp(Integer) (+ (.maxhp _superficialstatus) inValue) 0 10000)))
    (:NewEnumerator4
      ;[1 1 1] Resilienceの加算
      (設定|SetStatus "NewEnumerator4" (Math|Integer|Clamp(Integer) (+ (.resilience _superficialstatus) inValue) 0 500)))))

(fn PullStatus
  (params (serectName :type StatusName%20Enum :default "NewEnumerator0") (inValue :type Integer))
  (bind _superficialstatus (Variables|ステータス|GetsuperficialStatus))
  (switch Utilities|FlowControl|Switch|SwitchonStatusName serectName
    (:NewEnumerator0
      ;[1 1 1] Powerの加算
      (設定|SetStatus "NewEnumerator0" (Math|Integer|Clamp(Integer) (- (.power _superficialstatus) inValue) 0 100)))
    (:NewEnumerator1
      ;[1 1 1] MaxSpeedの加算
      (設定|SetStatus "NewEnumerator1" (Math|Integer|Clamp(Integer) (- (.maxspeed _superficialstatus) inValue) 0 100)))
    (:NewEnumerator2
      ;[1 1 1] Accelerationの加算
      (設定|SetStatus "NewEnumerator2" (Math|Integer|Clamp(Integer) (- (.acceleration _superficialstatus) inValue) 0 100)))
    (:NewEnumerator3
      ;[1 1 1] HPの加算
      (設定|SetStatus "NewEnumerator3" (Math|Integer|Clamp(Integer) (- (.maxhp _superficialstatus) inValue) 0 10000)))
    (:NewEnumerator4
      ;[1 1 1] Resilienceの加算
      (設定|SetStatus "NewEnumerator4" (Math|Integer|Clamp(Integer) (- (.resilience _superficialstatus) inValue) 0 500)))))