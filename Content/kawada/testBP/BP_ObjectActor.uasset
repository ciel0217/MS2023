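; Test movable object that knocks other BP_ObjectActors away on contact, with provisional flip logic.
; BeginPlay can load default Status from the BP_LevelMG game instance; MoveImpact feeds scaled input into FloatingPawnMovement.
; On capsule overlap, both objects' input-speed × RotSpeed scores set a lerped impulse on the other's mesh, cut sharply if this one scores lower.
; Hits show debug text and arrows; GetFlip is an empty stub.
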(event OnComponentBeginOverlap(Capsule)
  (params (OverlappedComponent :type Primitive%20Component%20Object%20Reference) (OtherActor :type Actor%20Object%20Reference) (OtherComp :type Primitive%20Component%20Object%20Reference) (OtherBodyIndex :type Integer) (bFromSweep :type Boolean) (SweepResult :type Hit%20Result%20Structure%20%28by%20ref%29))
  (bind _returnvalue (Transformation|GetActorLocation))
  (bind _status (Variables|Default|GetStatus))
  ;[1 1 1] 弾く仮実装
  (bind _asbp_object_actor (Utilities|Casting|CastToBP_ObjectActor OtherActor))
  (Variables|Default|SetactorLocation _returnvalue)
  (bind _output_get (Variables|Default|SetHitActor _asbp_object_actor))
  (bind _multires (CallFunction|GetStatus _output_get))
  (bind _multires_2 (CallFunction|GetStatus))
  (if (>= _multires_2 _multires)
    (Development|PrintString "hit")
    (Rendering|Debug|DrawDebugArrow (Variables|Default|GetactorLocation) (+ (* (Math|Vector|GetUnitDirection(Vector) _returnvalue (Transformation|GetActorLocation _asbp_object_actor)) (Math|Float|Lerp (.lowflippow _status) (.highflippow _status) (Math|Float|Clamp(Float) (/ (Math|Float|Absolute(Float) (- _multires _multires_2)) (.flipdisstatus _status))))) (Variables|Default|GetactorLocation)) 1.0 "(R=1.000000,G=0.107146,B=0.000000,A=1.000000)" 1.0 0.0)
    (CallFunction|ImpulseAction (Variables|Default|GetHitActor) (* (Math|Vector|GetUnitDirection(Vector) _returnvalue (Transformation|GetActorLocation _asbp_object_actor)) (Math|Float|Lerp (.lowflippow _status) (.highflippow _status) (Math|Float|Clamp(Float) (/ (Math|Float|Absolute(Float) (- _multires _multires_2)) (.flipdisstatus _status))))))
    (else
      (Development|PrintString "hit")
      (Rendering|Debug|DrawDebugArrow (Variables|Default|GetactorLocation) (+ (* (Math|Vector|GetUnitDirection(Vector) _returnvalue (Transformation|GetActorLocation _asbp_object_actor)) (* (Math|Float|Lerp (.lowflippow _status) (.highflippow _status) (Math|Float|Clamp(Float) (/ (Math|Float|Absolute(Float) (- _multires _multires_2)) (.flipdisstatus _status)))) 0.2)) (Variables|Default|GetactorLocation)) 1.0 "(R=0.000000,G=1.000000,B=0.013004,A=1.000000)" 1.0 0.0)
      (CallFunction|ImpulseAction (Variables|Default|GetHitActor) (* (Math|Vector|GetUnitDirection(Vector) _returnvalue (Transformation|GetActorLocation _asbp_object_actor)) (* (Math|Float|Lerp (.lowflippow _status) (.highflippow _status) (Math|Float|Clamp(Float) (/ (Math|Float|Absolute(Float) (- _multires _multires_2)) (.flipdisstatus _status)))) 0.2)))))
  (CallFunction|GetFlip))

(event Custom|MoveImpact
  (params (ImpactParam :type Vector))
  ;[1 1 1] 移動関数
  (Class|PawnMovementComponent|AddInputVector (Variables|Default|GetFloatingPawnMovement) (* ImpactParam (* (.defaultvec (Variables|Default|GetStatus)) (Variables|Default|GetSpeed))) false))

(event EventBeginPlay
  (if (Variables|Default|GetDefaultStatus)
    (bind _asgame_instance (Utilities|Casting|CastToGameInstance (Game|GetGameInstance)))
    (bind _asbp_level_mg (Utilities|Casting|CastToBP_LevelMG _asgame_instance))
    (bind _defaultstatus (Default|GetDefaultStatus _asbp_level_mg))
    (Variables|Default|SetStatus _defaultstatus)))

(event Collision|EventActorBeginOverlap
  (params (OtherActor :type Actor%20Object%20Reference)))

(fn ConstructionScript)

(fn GetStatus
  (bind _status (Variables|Default|GetStatus))
  (bind _rotspeed (Variables|Default|GetRotSpeed))
  (bind _floatingpawnmovement (Variables|Default|GetFloatingPawnMovement))
  (bind _returnvalue (Pawn|Components|PawnMovement|GetLastInputVector _floatingpawnmovement))
  (bind _returnvalue_2 (Math|Vector|VectorLength _returnvalue))
  (bind _returnvalue_3 (/ _returnvalue_2 (.defaultvec _status)))
  (bind _returnvalue_4 (+ _returnvalue_3 1.0))
  (return _returnvalue_4 _rotspeed (* _returnvalue_4 _rotspeed)))

(fn ImpulseAction
  (params (PalseValue :type Vector))
  (Physics|AddImpulse (Variables|Default|GetSM_moveObject) PalseValue "None" true))

(fn GetFlip)