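; Storm spark effect actor that draws a jumping lightning beam between two groups of scene points.
; BeginPlay gathers six components into start and end arrays, and every Tick picks a random point from each.
; SetThunderLocation feeds their world positions into the NSSpark Niagara beam, plus distance as cylinder height and look-at pitch (offset 90 degrees) and yaw to orient it.
; The particle data callback is empty and its owner binding never runs.
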(event EventBeginPlay
  (Variables|Default|SetStorm01 (Utilities|Array|MakeArray (Variables|Default|Get01) (Variables|Default|Get02) (Variables|Default|Get03)))
  (Variables|Default|SetStorm02 (Utilities|Array|MakeArray (Variables|Default|Get04) (Variables|Default|Get05) (Variables|Default|Get06))))

(event Collision|EventActorBeginOverlap
  (params (OtherActor :type Actor%20Object%20Reference)))

(event EventTick
  (params (DeltaSeconds :type Float%20%28single-precision%29))
  (CallFunction|SetThunderLocation (Variables|Default|GetNS_Spark) (Variables|Default|GetStorm01) (Variables|Default|GetStorm02)))

(event EventParticleData
  (params (Data :type Array%20of%20Basic%20Particle%20Data%20Structures) (NiagaraSystem :type Niagara%20System%20Object%20Reference) (SimulationPositionOffset :type Vector%20%28by%20ref%29 :default "0, 0, 0")))

(fn ConstructionScript)

(fn SetThunderLocation
  (params (Naiagara :type Niagara%20Component%20Object%20Reference) (Start :type Array%20of%20Scene%20Component%20Object%20References) (End :type Array%20of%20Scene%20Component%20Object%20References))
  (bind _output_get (Variables|Default|SetRight%20Start (Transformation|GetWorldLocation (Utilities|Array|Get(acopy) Start (Math|Random|RandomIntegerinRange 0 (Utilities|Array|LastIndex Start))))))
  (bind _output_get_2 (Variables|Default|SetRight%20End (Transformation|GetWorldLocation (Utilities|Array|Get(acopy) End (Math|Random|RandomIntegerinRange 0 (Utilities|Array|LastIndex End))))))
  (Niagara|SetNiagaraVariable(Vector3) Naiagara "Beam Start" _output_get)
  (Niagara|SetNiagaraVariable(Vector3) Naiagara "Beam End" _output_get_2)
  (Niagara|SetNiagaraVariable(Float) Naiagara "Cylinder Height" (Math|Vector|Distance(Vector) (Variables|Default|GetRight%20Start) (Variables|Default|GetRight%20End)))
  (Niagara|SetNiagaraVariable(Float) Naiagara "Pitch" (+ (.pitch (Math|Rotator|FindLookatRotation (Variables|Default|GetRight%20Start) (Variables|Default|GetRight%20End))) -9e+01))
  (Niagara|SetNiagaraVariable(Float) Naiagara "Yaw" (.yaw (Math|Rotator|FindLookatRotation (Variables|Default|GetRight%20Start) (Variables|Default|GetRight%20End)))))