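; Breakable wooden box actor, in a test folder, that extends a parent break object and drops a random item when broken.
; It supplies six plate components as the parent's mesh array and always returns true from IsAngle.
; Break runs the parent logic, plays a wood-break sound, then spawns the item offset along the player's forward vector.
; The item's Box gets physics and a random, upward-biased impulse scaled by Power.
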(event EventBeginPlay
  (|CallParentFunction) ; このノードは無効になっているため呼び出せません。\n機能をビルドするにはピンをドラッグしてください。
)

(event Collision|EventActorBeginOverlap
  (params (OtherActor :type Actor%20Object%20Reference))
  (|CallParentFunction OtherActor) ; このノードは無効になっているため呼び出せません。\n機能をビルドするにはピンをドラッグしてください。
)

(event EventTick
  (params (DeltaSeconds :type Float%20%28single-precision%29))
  (|CallParentFunction DeltaSeconds) ; このノードは無効になっているため呼び出せません。\n機能をビルドするにはピンをドラッグしてください。
)

(fn ConstructionScript
  (|CallParentFunction))

(fn CreateMeshArray
  (Variables|Default|SetMeshArray (Utilities|Array|MakeArray (Variables|Default|GetPlate3) (Variables|Default|GetPlate4) (Variables|Default|GetPlate5) (Variables|Default|GetPlate) (Variables|Default|GetPlate1) (Variables|Default|GetPlate2))))

(fn IsAngle
  (return true))

(fn IsOP)

(fn Break
  (bind _returnvalue (Math|Random|RandomUnitVector))
  (bind _returnvalue_2 (Transformation|GetActorTransform))
  (bind _power (Variables|Default|Getpower))
  (|CallParentFunction)
  (Audio|PlaySoundatLocation "/Game/kawada/Sound/WoodBreak_Cue.WoodBreak_Cue" (Transformation|GetActorLocation) "0, 0, 0" 0.25 1.0 0.025 0 "/Game/okada/SE/NewSoundConcurrency.NewSoundConcurrency" 0 0)
  (bind _returnvalue_3 (Game|SpawnActorfromClass (.OutItem (Utilities|Array|Random (Variables|Default|GetItems))) (Math|Transform|MakeTransform (+ (.location _returnvalue_2) (* (Transformation|GetActorForwardVector (Game|Player|GetPlayerPawn 0)) "100.000000,100.000000,10.000000")) (.rotation _returnvalue_2) "1.000000,1.000000,1.000000") "Undefined" "MultiplyWithRoot" 0 0))
  (Utilities|IsValid (Variables|/Game/Ishikawa/Item/BP_BaseItem.BP_BaseItem_C|GetBox _returnvalue_3)
    (:Is%20Valid
      (Physics|SetSimulatePhysics (Variables|/Game/Ishikawa/Item/BP_BaseItem.BP_BaseItem_C|GetBox _returnvalue_3) true)
      (Physics|AddImpulse (Variables|/Game/Ishikawa/Item/BP_BaseItem.BP_BaseItem_C|GetBox _returnvalue_3) (Math|Vector|MakeVector (* (.x _returnvalue) _power) (* (.y _returnvalue) _power) (* (Math|Float|Absolute(Float) (.z _returnvalue)) (/ _power 2.0))) "None" true))))