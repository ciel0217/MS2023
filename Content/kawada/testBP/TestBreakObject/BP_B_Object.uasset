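; Breakable obstacle Blueprint that shatters when a BP_ObjectActor hits its Box at a steep enough angle and high enough speed.
; On a valid hit it destroys the Box, turns on physics for each MeshArray piece and impulses it away from the actor.
; It bounces the actor off by mirroring its velocity, briefly disables its control, then destroys itself after a delay.
; CreateMeshArray is an empty stub here.
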(event OnComponentBeginOverlap(Box)
  (params (OverlappedComponent :type Primitive%20Component%20Object%20Reference) (OtherActor :type Actor%20Object%20Reference) (OtherComp :type Primitive%20Component%20Object%20Reference) (OtherBodyIndex :type Integer) (bFromSweep :type Boolean) (SweepResult :type Hit%20Result%20Structure%20%28by%20ref%29))
  (bind _asbp_object_actor (Utilities|Casting|CastToBP_ObjectActor OtherActor))
  (Variables|Default|SetAs%20BP%20Object%20Actor _asbp_object_actor)
  (bind _returnvalue (CallFunction|IsAngle))
  (if _returnvalue
    (bind _returnvalue_2 (CallFunction|IsSpeed))
    (if _returnvalue_2
      (Components|DestroyComponent (Variables|Default|GetBox))
      (for _array_element (Variables|Default|GetMeshArray)
        (Physics|SetSimulatePhysics _array_element true)
        (Physics|AddImpulse _array_element (Math|Vector|MakeVector (.x (* (Math|Vector|Normalize (- (Transformation|GetWorldLocation _array_element) (Transformation|GetActorLocation (Variables|Default|GetAs%20BP%20Object%20Actor)))) 1e+03)) (.y (* (Math|Vector|Normalize (- (Transformation|GetWorldLocation _array_element) (Transformation|GetActorLocation (Variables|Default|GetAs%20BP%20Object%20Actor)))) 1e+03)) (* (.z (* (Math|Vector|Normalize (- (Transformation|GetWorldLocation _array_element) (Transformation|GetActorLocation (Variables|Default|GetAs%20BP%20Object%20Actor)))) 1e+03)) 0.2)) "None" true))
      (Default|ImpulseAction (Variables|Default|GetAs%20BP%20Object%20Actor) (* (Math|Vector|MirrorVectorbyNormal (+ (Transformation|GetComponentVelocity (Variables|/Game/kawada/testBP/TestMoveObject/BP_ObjectActor.BP_ObjectActor_C|GetSM_moveObject (Variables|Default|GetAs%20BP%20Object%20Actor))) (Variables|/Game/kawada/testBP/TestMoveObject/BP_ObjectActor.BP_ObjectActor_C|GetinVelocity (Variables|Default|GetAs%20BP%20Object%20Actor))) (Transformation|GetActorRightVector)) (Variables|Default|GetReflectMag)))
      (CallFunction|DeleteObject))))

(event Custom|DeleteObject
  (CallFunction|IsOP)
  (Utilities|FlowControl|Delay 3.0)
  (Actor|DestroyActor))

(event EventBeginPlay
  (CallFunction|CreateMeshArray))

(event Collision|EventActorBeginOverlap
  (params (OtherActor :type Actor%20Object%20Reference)))

(event EventTick
  (params (DeltaSeconds :type Float%20%28single-precision%29)))

(fn ConstructionScript)

(fn Dead
  (Actor|DestroyActor))

(fn CreateMeshArray)

(fn IsAngle
  (bind _as_bp_object_actor (Variables|Default|GetAs%20BP%20Object%20Actor))
  (return (>= (Math|Float|Absolute(Float) (Math|Vector|DotProduct (Math|Vector|Normalize (+ (Variables|/Game/kawada/testBP/TestMoveObject/BP_ObjectActor.BP_ObjectActor_C|GetinVelocity _as_bp_object_actor) (Transformation|GetComponentVelocity (Variables|/Game/kawada/testBP/TestMoveObject/BP_ObjectActor.BP_ObjectActor_C|GetSM_moveObject _as_bp_object_actor)))) (Transformation|GetActorRightVector))) 0.65)))

(fn IsSpeed
  (bind _as_bp_object_actor (Variables|Default|GetAs%20BP%20Object%20Actor))
  (return (>= (/ (Math|Vector|VectorLength (+ (Transformation|GetComponentVelocity (Variables|/Game/kawada/testBP/TestMoveObject/BP_ObjectActor.BP_ObjectActor_C|GetSM_moveObject _as_bp_object_actor)) (Variables|/Game/kawada/testBP/TestMoveObject/BP_ObjectActor.BP_ObjectActor_C|GetinVelocity _as_bp_object_actor))) (Class|MovementComponent|GetMaxSpeed (Variables|/Game/kawada/testBP/TestMoveObject/BP_ObjectActor.BP_ObjectActor_C|GetFloatingPawnMovement (Variables|Default|GetAs%20BP%20Object%20Actor)))) (Variables|Default|GetBreakSpeed))))

(fn IsOP
  (bind _as_bp_object_actor (Variables|Default|GetAs%20BP%20Object%20Actor))
  (Variables|/Game/kawada/testBP/TestMoveObject/BP_ObjectActor.BP_ObjectActor_C|SetisOperation _as_bp_object_actor false)
  (Utilities|Time|SetTimerbyFunctionName _as_bp_object_actor "NC_Inoperable" 0.1)
  (return))