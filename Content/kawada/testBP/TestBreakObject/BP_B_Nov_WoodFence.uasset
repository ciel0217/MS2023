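; BP_B_Nov_WoodFence is a wooden fence Blueprint in a break-object test folder, built from six wood mesh pieces.
; CreateMeshArray fills MeshArray with those pieces, the Wood and LandWood components.
; The construction script only calls the parent's, and BeginPlay, overlap and Tick are disabled stubs, so the asset adds no event logic of its own.
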(event EventBeginPlay
  (|CallParentFunction) ; このノードは無効になっているため呼び出せません。\n機能をビルドするにはピンをドラッグしてください。
)

(event Collision|EventActorBeginOverlap
  (params (OtherActor :type Actor%20Object%20Reference))
  (|CallParentFunction OtherActor) ; このノードは無効になっているため呼び出せません。\n機能をビルドするにはピンをドラッグしてください。
)

(event EventTick
  (params (DeltaSeconds :type Float%20%28single-precision%29))
  (|CallParentFunction DeltaSeconds) ; このノードは無効になっているため呼び出せません。\n機能をビルドするにはピンをドラッグしてください。
)

(fn ConstructionScript
  (|CallParentFunction))

(fn CreateMeshArray
  (Variables|Default|SetMeshArray (Utilities|Array|MakeArray (Variables|Default|GetWood2) (Variables|Default|GetWood1) (Variables|Default|GetLandWood2) (Variables|Default|GetLandWood1) (Variables|Default|GetWood4) (Variables|Default|GetWood3))))