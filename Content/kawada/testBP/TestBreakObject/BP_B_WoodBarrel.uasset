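; Wooden barrel Blueprint in a break-object test folder, apparently a child of a shared breakable-object parent.
; It supplies per-object data through functions: CreateMeshArray fills MeshArray with six plate pieces, and IsAngle always returns true.
; IsOP is empty, the construction script only calls the parent, and the event graph holds only disabled stub events, leaving any break behavior outside this file.
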(event EventBeginPlay
  (|CallParentFunction) ; このノードは無効になっているため呼び出せません。\n機能をビルドするにはピンをドラッグしてください。
)

(event Collision|EventActorBeginOverlap
  (params (OtherActor :type Actor%20Object%20Reference))
  (|CallParentFunction OtherActor) ; このノードは無効になっているため呼び出せません。\n機能をビルドするにはピンをドラッグしてください。
)

(event EventTick
  (params (DeltaSeconds :type Float%20%28single-precision%29))
  (|CallParentFunction DeltaSeconds) ; このノードは無効になっているため呼び出せません。\n機能をビルドするにはピンをドラッグしてください。
)

(fn ConstructionScript
  (|CallParentFunction))

(fn CreateMeshArray
  (Variables|Default|SetMeshArray (Utilities|Array|MakeArray (Variables|Default|GetPlate2) (Variables|Default|GetPlate1) (Variables|Default|GetPlate6) (Variables|Default|GetPlate5) (Variables|Default|GetPlate) (Variables|Default|GetPlate3))))

(fn IsAngle
  (return true))

(fn IsOP)